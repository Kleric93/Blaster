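; Player character Blueprint for a Blaster shooter, handling local UI, audio toggles and a taunt.
; After a short BeginPlay delay it shows the player's name on the overhead widget.
; Sniper and M4 scope events lazily create their widgets, playing zoom animations forward or reversed with sounds.
; Input toggles music and master mute sound mixes, opens or closes the pause menu, and plays the taunt montage through RPC-named events.
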(event `InputAction|MuteMusic`
  (params (Key :type "Key Structure"))
  (:`Pressed`
    (`/Engine/EditorBlueprintResources/StandardMacros.FlipFlop`
      (:`A`
        (`GameplayStatics.SetBaseSoundMix` "/Game/Assets/Sounds/SoundClassesnMixes/SCM_Mute_Music.SCM_Mute_Music"))
      (:`B`
        (`GameplayStatics.SetBaseSoundMix` "/Game/Assets/Sounds/SoundClassesnMixes/SCM_UnMute_MUsic.SCM_UnMute_MUsic")))))

(event `InputAction|Mute/Unmute`
  (params (Key :type "Key Structure"))
  (:`Pressed`
    (`/Engine/EditorBlueprintResources/StandardMacros.FlipFlop`
      (:`A`
        (`GameplayStatics.SetBaseSoundMix` "/Game/Assets/Sounds/SoundClassesnMixes/SCM_Mute_MasterClass.SCM_Mute_MasterClass"))
      (:`B`
        (`GameplayStatics.SetBaseSoundMix` "/Game/Assets/Sounds/SoundClassesnMixes/SCM_UnMute_MasterClass.SCM_UnMute_MasterClass")))))

(event `self.ReceiveBeginPlay`
  (`KismetSystemLibrary.Delay` 2.0)
  (bind _aswbp_overhead_widget (cast `/Game/Blueprints/HUD/WBP_OverheadWidget` (`WidgetComponent.GetUserWidgetObject` (`self.OverheadWidget`))))
  (`OverheadWidget.ShowPlayerName` _aswbp_overhead_widget self))

(event `self.ReceiveTick`
  (params (DeltaSeconds :type "Float (single-precision)")))

(event `EnhancedInput|/Game/Blueprints/InputActions/Actions/IA_Pause`
  (params (ActionValue :type Boolean) (ElapsedSeconds :type "Float (double-precision)") (TriggeredSeconds :type "Float (double-precision)") (InputAction :type "InputAction Object Reference" :default "/Game/Blueprints/InputActions/Actions/IA_Pause.IA_Pause"))
  (bind _returnvalue (`GameplayStatics.GetPlayerController` 0))
  ;[0.01096 0.01161 0.0137] PauseMenu
  (:`Started`
    (if (not (`self.bIsMenuVisible`))
      (set `self.bIsMenuVisible` true)
      (bind _returnvalue_2 (`|CreateWidget` "/Game/Blueprints/HUD/WBP_ReturnToMainMenu.WBP_ReturnToMainMenu_C" _returnvalue))
      (bind _output_get (set `self.PauseMenuWidget` _returnvalue_2))
      (`UserWidget.AddToViewport` _output_get 0)
      (`WidgetBlueprintLibrary.SetInputMode_GameAndUIEx` null null)
      (`self.DisableInput` _returnvalue)
      (else
        (set `self.bIsMenuVisible` false)
        (`Widget.RemoveFromParent` (`self.PauseMenuWidget`))
        (`self.EnableInput` _returnvalue)))))

(event `self.ShowSniperScopeWidget`
  (params (bShowScope :type Boolean))
  (bind _sniperscopewidget (`self.SniperScopeWidget`))
  (`/Engine/EditorBlueprintResources/StandardMacros.IsValid` (`self.SniperScopeWidget`)
    (:`Is Valid`
      _)
    (:`Is Not Valid`
      (bind _returnvalue (`|CreateWidget` "/Game/Blueprints/HUD/WBP_SniperScope.WBP_SniperScope_C"))
      (bind _output_get (set `self.SniperScopeWidget` _returnvalue))
      (`UserWidget.AddToViewport` _output_get 0)))
  (if bShowScope
    ;[0.01096 0.01161 0.0137] PauseMenu
    (`/Engine/EditorBlueprintResources/StandardMacros.IsValid` _sniperscopewidget
      (:`Is Valid`
        (`UserWidget.PlayAnimation` _sniperscopewidget (`/Game/Blueprints/HUD/WBP_SniperScope.ScopeZoomIn` _sniperscopewidget) 0.0 1 "Forward" 1.0 false)
        (`GameplayStatics.PlaySound2D` "/Game/Assets/MilitaryWeapSilver/Sound/SniperRifle/Wavs/SniperRifle_ZoomIn.SniperRifle_ZoomIn" 1.0 1.0 0.0 null null)))
    (else
      (`/Engine/EditorBlueprintResources/StandardMacros.IsValid` _sniperscopewidget
        (:`Is Valid`
          (`UserWidget.PlayAnimation` _sniperscopewidget (`/Game/Blueprints/HUD/WBP_SniperScope.ScopeZoomIn` _sniperscopewidget) 0.0 1 "Reverse" 1.0 false)
          (`GameplayStatics.PlaySound2D` "/Game/Assets/MilitaryWeapSilver/Sound/SniperRifle/Wavs/SniperRifle_ZoomOut.SniperRifle_ZoomOut" 1.0 1.0 0.0 null null))))))

(event `self.ShowM4ScopeWidget`
  (params (bShowScope :type Boolean))
  (bind _m4scopewidget (`self.M4ScopeWidget`))
  (`/Engine/EditorBlueprintResources/StandardMacros.IsValid` (`self.M4ScopeWidget`)
    (:`Is Valid`
      _)
    (:`Is Not Valid`
      (bind _returnvalue (`|CreateWidget` "/Game/Blueprints/HUD/WBP_M4Scope.WBP_M4Scope_C"))
      (bind _output_get (set `self.M4ScopeWidget` _returnvalue))
      (`UserWidget.AddToViewport` _output_get 0)))
  (if bShowScope
    (`/Engine/EditorBlueprintResources/StandardMacros.IsValid` _m4scopewidget
      (:`Is Valid`
        (`UserWidget.PlayAnimation` _m4scopewidget (`/Game/Blueprints/HUD/WBP_M4Scope.M4ScopeZoom` _m4scopewidget) 0.0 1 "Forward" 1.0 false)
        (`GameplayStatics.PlaySound2D` "/Game/Assets/M4AZ/Sounds/ZoomIn_Cue.ZoomIn_Cue" 1.0 1.0 0.0 null null)))
    (else
      (`/Engine/EditorBlueprintResources/StandardMacros.IsValid` _m4scopewidget
        (:`Is Valid`
          (`UserWidget.PlayAnimation` _m4scopewidget (`/Game/Blueprints/HUD/WBP_M4Scope.M4ScopeZoom` _m4scopewidget) 0.0 1 "Reverse" 2.0 false)
          (`GameplayStatics.PlaySound2D` "/Game/Assets/M4AZ/Sounds/ZoomOut_Cue.ZoomOut_Cue" 1.0 1.0 0.0 null null))))))

(event `InputAction|Taunt`
  (params (Key :type "Key Structure"))
  (:`Pressed`
    (`self.RPC Play Animation`)))

(event `RPC Play Animation`
  (`self.Play Animation`))

(event `Play Animation`
  (`self.PlayAnimMontage` "/Game/Blueprints/Animation/AM_TauntAnimMontage.AM_TauntAnimMontage" 1.3))

(fn `NewFunction`
  (params (self2 :type "MovementComponent Object Reference"))
  (`MovementComponent.StopMovementImmediately` self2))

(fn `UserConstructionScript`)