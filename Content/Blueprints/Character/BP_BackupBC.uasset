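; Player character Blueprint, apparently a backup, that handles sniper and M4 scope overlays and a taunt.
; The scope events lazily create and cache their widgets, playing zoom animations forward or in reverse with matching sounds.
; Taunt input plays a montage through an RPC-named event chain.
; Overhead name, net role and input mapping setup are disconnected, and Tick and BeginPlay are empty.
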(event `self.ReceiveBeginPlay`)

(event `self.ReceiveTick`
  (params (DeltaSeconds :type "Float (single-precision)")))

(event `self.ShowSniperScopeWidget`
  (params (bShowScope :type Boolean))
  (bind _sniperscopewidget (`self.SniperScopeWidget`))
  (`/Engine/EditorBlueprintResources/StandardMacros.IsValid` (`self.SniperScopeWidget`)
    (:`Is Valid`
      _)
    (:`Is Not Valid`
      (bind _returnvalue (`|CreateWidget` "/Game/Blueprints/HUD/WBP_SniperScope.WBP_SniperScope_C"))
      (bind _output_get (set `self.SniperScopeWidget` _returnvalue))
      (`UserWidget.AddToViewport` _output_get 0)))
  (if bShowScope
    (`/Engine/EditorBlueprintResources/StandardMacros.IsValid` _sniperscopewidget
      (:`Is Valid`
        (`UserWidget.PlayAnimation` _sniperscopewidget (`/Game/Blueprints/HUD/WBP_SniperScope.ScopeZoomIn` _sniperscopewidget) 0.0 1 "Forward" 1.0 false)
        (`GameplayStatics.PlaySound2D` "/Game/Assets/MilitaryWeapSilver/Sound/SniperRifle/Wavs/SniperRifle_ZoomIn.SniperRifle_ZoomIn" 1.0 1.0 0.0 null null)))
    (else
      (`/Engine/EditorBlueprintResources/StandardMacros.IsValid` _sniperscopewidget
        (:`Is Valid`
          (`UserWidget.PlayAnimation` _sniperscopewidget (`/Game/Blueprints/HUD/WBP_SniperScope.ScopeZoomIn` _sniperscopewidget) 0.0 1 "Reverse" 1.0 false)
          (`GameplayStatics.PlaySound2D` "/Game/Assets/MilitaryWeapSilver/Sound/SniperRifle/Wavs/SniperRifle_ZoomOut.SniperRifle_ZoomOut" 1.0 1.0 0.0 null null))))))

(event `self.ShowM4ScopeWidget`
  (params (bShowScope :type Boolean))
  (bind _m4scopewidget (`self.M4ScopeWidget`))
  (`/Engine/EditorBlueprintResources/StandardMacros.IsValid` (`self.M4ScopeWidget`)
    (:`Is Valid`
      _)
    (:`Is Not Valid`
      (bind _returnvalue (`|CreateWidget` "/Game/Blueprints/HUD/WBP_M4Scope.WBP_M4Scope_C"))
      (bind _output_get (set `self.M4ScopeWidget` _returnvalue))
      (`UserWidget.AddToViewport` _output_get 0)))
  (if bShowScope
    (`/Engine/EditorBlueprintResources/StandardMacros.IsValid` _m4scopewidget
      (:`Is Valid`
        (`UserWidget.PlayAnimation` _m4scopewidget (`/Game/Blueprints/HUD/WBP_M4Scope.M4ScopeZoom` _m4scopewidget) 0.0 1 "Forward" 1.0 false)
        (`GameplayStatics.PlaySound2D` "/Game/Assets/M4AZ/Sounds/ZoomIn_Cue.ZoomIn_Cue" 1.0 1.0 0.0 null null)))
    (else
      (`/Engine/EditorBlueprintResources/StandardMacros.IsValid` _m4scopewidget
        (:`Is Valid`
          (`UserWidget.PlayAnimation` _m4scopewidget (`/Game/Blueprints/HUD/WBP_M4Scope.M4ScopeZoom` _m4scopewidget) 0.0 1 "Reverse" 2.0 false)
          (`GameplayStatics.PlaySound2D` "/Game/Assets/M4AZ/Sounds/ZoomOut_Cue.ZoomOut_Cue" 1.0 1.0 0.0 null null))))))

(event `InputAction|Taunt`
  (params (Key :type "Key Structure"))
  (:`Pressed`
    (`self.RPC Play Animation`)))

(event `RPC Play Animation`
  (`self.Play Animation`))

(event `Play Animation`
  (`self.PlayAnimMontage` "/Game/Blueprints/Animation/AM_TauntAnimMontage.AM_TauntAnimMontage" 1.3))

(fn `NewFunction`
  (params (self2 :type "MovementComponent Object Reference"))
  (`MovementComponent.StopMovementImmediately` self2))

(fn `UserConstructionScript`)