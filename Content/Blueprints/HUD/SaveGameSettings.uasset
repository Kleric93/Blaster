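; SaveGameSettings stores the player's graphics options for the HUD settings, apparently as a save game object.
; It holds a console command and a selected setting enum for each category: overall graphics, shadows, anti-aliasing, post-processing, textures, view distance and effects.
; SetSettings writes all values at once, while ReturnCommands and ReturnEnums read back the commands and enum selections separately.
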(fn `ReturnCommands`
  (returns (GraphicsCommand :type String) (ShadowCommand :type String) (AACommand :type String) (PPCommand :type String) (TextureCommand :type String) (DistanceCOmmand :type String) (EffectCommand :type String))
  (return (`self.GraphicsCommand`) (`self.ShadowCommand`) (`self.AACommand`) (`self.PPCommand`) (`self.TextureCommand`) (`self.DistanceCOmmand`) (`self.EffectCommand`)))

(fn `ReturnEnums`
  (returns (GraphicSettings :type "/Game/Blueprints/HUD/p Enum") (ShadowSetting :type "/Game/Blueprints/HUD/p Enum") (AASetting :type "/Game/Blueprints/HUD/p Enum") (PPSetting :type "/Game/Blueprints/HUD/p Enum") (TextureSetting :type "/Game/Blueprints/HUD/p Enum") (DistanceSetting :type "/Game/Blueprints/HUD/p Enum") (EffectSetting :type "/Game/Blueprints/HUD/p Enum"))
  (return (`self.GraphicSettings`) (`self.ShadowSetting`) (`self.AASetting`) (`self.PPSetting`) (`self.TextureSetting`) (`self.DistanceSetting`) (`self.EffectSetting`)))

(fn `SetSettings`
  (params (`Graphics Command` :type String) (ShadowCommand1 :type String) (AACommand :type String) (PPCommand :type String) (TextureCommand :type String) (DistanceCOmmand :type String) (EffectCommand :type String) (GraphicSettings :type "/Game/Blueprints/HUD/p Enum" :default "NewEnumerator0") (ShadowSetting :type "/Game/Blueprints/HUD/p Enum" :default "NewEnumerator0") (AASetting :type "/Game/Blueprints/HUD/p Enum" :default "NewEnumerator0") (PPSetting :type "/Game/Blueprints/HUD/p Enum" :default "NewEnumerator0") (TextureSetting :type "/Game/Blueprints/HUD/p Enum" :default "NewEnumerator0") (DistanceSetting :type "/Game/Blueprints/HUD/p Enum" :default "NewEnumerator0") (EffectSetting :type "/Game/Blueprints/HUD/p Enum" :default "NewEnumerator0"))
  (set `self.GraphicsCommand` `Graphics Command`)
  (set `self.ShadowCommand` ShadowCommand1)
  (set `self.AACommand` AACommand)
  (set `self.PPCommand` PPCommand)
  (set `self.TextureCommand` TextureCommand)
  (set `self.DistanceCOmmand` DistanceCOmmand)
  (set `self.EffectCommand` EffectCommand)
  (set `self.GraphicSettings` GraphicSettings)
  (set `self.ShadowSetting` ShadowSetting)
  (set `self.AASetting` AASetting)
  (set `self.PPSetting` PPSetting)
  (set `self.TextureSetting` TextureSetting)
  (set `self.DistanceSetting` DistanceSetting)
  (set `self.EffectSetting` EffectSetting))